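; Player character that can board nearby SCBP_Pawn vehicles as either driver or gunner.
; Pressing I sphere-traces for the closest vehicle, with debug drawing left on.
; A vehicle without a player controller gets possessed while the character hides; a player-driven one has the character attached at GunnerSocket with movement and collision off.
; Pressing O leaves the gunner seat, using the saved relative offset to reposition and restoring walking and collision.
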(event `self.ReceiveBeginPlay`
  (`parent.ReceiveBeginPlay`)
  (bind _asplayer_controller (cast `PlayerController` (`self.GetController`)))
  (set `self.PreviousPlayerController` _asplayer_controller))

(event `Key|I`
  (params (Key :type "Key Structure"))
  (:`Pressed`
    (`self.OnEnterVehicle` null)))

(event `Key|O`
  (params (Key :type "Key Structure"))
  (:`Pressed`
    (if (not (`self.CanMove`))
      (`self.K2_DetachFromActor` "KeepWorld" "KeepWorld")
      (`self.K2_SetActorLocation` (- (`self.K2_GetActorLocation`) (`self.PreviousRelPawnPosition`)) false true)
      (set `self.CanMove` true)
      (`CharacterMovementComponent.SetMovementMode` (`self.CharacterMovement`) "MOVE_Walking" 0)
      (`PrimitiveComponent.SetCollisionEnabled` (`self.CapsuleComponent`) "QueryAndPhysics"))))

(event `OnEnterVehicle`
  (params (Pawn :type "Pawn Object Reference"))
  (bind (_vehicle _success _playercontrolled) (`self.CheckForVehicle`))
  (if _success
    (if _playercontrolled
      (set `self.PreviousRelPawnPosition` (- (`self.K2_GetActorLocation` _vehicle) (`self.K2_GetActorLocation`)))
      (`CharacterMovementComponent.SetMovementMode` (`self.CharacterMovement`) "MOVE_None" 0)
      (`PrimitiveComponent.SetCollisionEnabled` (`self.CapsuleComponent`) "NoCollision")
      (bind _returnvalue (`self.K2_AttachToActor` _vehicle "GunnerSocket" "SnapToTarget" "SnapToTarget" "KeepRelative" false))
      (set `self.CanMove` (not _returnvalue))
      (else
        (bind _asscbp_pawn (cast `/Game/Blueprints/Pawns/SCBP_Pawn` _vehicle))
        (`self.SetActorHiddenInGame` true)
        (bind _asplayer_controller (cast `PlayerController` (`self.GetController`)))
        (`Controller.Possess` _asplayer_controller _asscbp_pawn)
        (`/Game/Blueprints/Pawns/SCBP_Pawn.OnClientEnterVehicle` _asscbp_pawn)))))

(fn `CheckForVehicle`
  (returns (Vehicle :type "Actor Object Reference") (Success :type Boolean) (PlayerControlled :type Boolean))
  (locals (ClosestVehicle :type "Actor Object Reference"))
  (bind _returnvalue (`self.K2_GetActorLocation`))
  (set `local.ClosestVehicle` null)
  (bind (_outhits _returnvalue_2) (`KismetSystemLibrary.SphereTraceMulti` :`Start` _returnvalue :`End` _returnvalue :`Radius` 200.0 :`TraceChannel` "TraceTypeQuery1" :`DrawDebugType` "ForDuration" :`DrawTime` 8.0))
  (if _returnvalue_2
    (for _array_element _outhits
      (bind (_bblockinghit _binitialoverlap _time _distance _location _impactpoint _normal _impactnormal _physmat _hitactor) (`GameplayStatics.BreakHitResult` _array_element))
      (if (`KismetMathLibrary.ClassIsChildOf` (`GameplayStatics.GetObjectClass` _hitactor) "/Game/Blueprints/Pawns/SCBP_Pawn.SCBP_Pawn_C")
        (`local.ClosestVehicle`
          (:`then`
            (if (< (`self.GetSquaredDistanceTo` self _hitactor) (`self.GetSquaredDistanceTo` self (`local.ClosestVehicle`)))
              (set `local.ClosestVehicle` _hitactor :!label _label)))
          (:`else`
            (goto _label))))))
  (bind _closestvehicle (`local.ClosestVehicle`)
    (:`then`
      (bind _asscbp_pawn (cast `/Game/Blueprints/Pawns/SCBP_Pawn` _closestvehicle)
        (:`then`
          (bind _returnvalue_3 (`self.GetController` _asscbp_pawn))
          (`/Engine/EditorBlueprintResources/StandardMacros.IsValid` _returnvalue_3
            (:`Is Valid`
              (if (`Controller.IsPlayerController` _returnvalue_3)
                (return _closestvehicle true true)
                (else
                  _)))
            (:`Is Not Valid`
              _))
          (return _closestvehicle true false))
        (:`CastFailed`
          _)))
    (:`else`
      _))
  (return null false false))

(fn `UserConstructionScript`
  (`parent.UserConstructionScript`))