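; SCBP_Pawn is a vehicle pawn that handles entering and exiting by switching control between itself and the player's character.
; The enter event adds its Enhanced Input mapping context to the controller.
; Pressing O finds the TPCBP_Pawn whose stored PreviousPlayerController matches the current controller.
; Exit then removes the mapping, teleports that character to the vehicle's left, unhides it and possesses it.
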(event `Key|O`
  (params (Key :type "Key Structure"))
  (:`Pressed`
    (bind (_pawn _success) (`self.GetPreviousCharacter`))
    (if _success
      (`self.OnClientExitVehicle` _pawn))))

(event `OnClientEnterVehicle`
  (bind _asplayer_controller (cast `PlayerController` (`self.GetController`)))
  (bind _returnvalue (pcsubsystem `EnhancedInputLocalPlayerSubsystem` _asplayer_controller))
  (`/Engine/EditorBlueprintResources/StandardMacros.IsValid` _returnvalue
    (:`Is Valid`
      (`EnhancedInputSubsystemInterface.AddMappingContext` _returnvalue "/Game/VehicleTemplate/Input/IMC_Default.IMC_Default" 0 (struct)))))

(event `OnClientExitVehicle`
  (params (Pawn :type "/Game/Blueprints/Pawns/TPCBP_Pawn Object Reference"))
  (bind _asplayer_controller (cast `PlayerController` (`self.GetController`)))
  (bind _returnvalue (pcsubsystem `EnhancedInputLocalPlayerSubsystem` _asplayer_controller))
  (`/Engine/EditorBlueprintResources/StandardMacros.IsValid` _returnvalue
    (:`Is Valid`
      (`EnhancedInputSubsystemInterface.RemoveMappingContext` _returnvalue "/Game/VehicleTemplate/Input/IMC_Default.IMC_Default" (struct))
      (`self.OnPossessCharacter` Pawn))))

(event `OnPossessCharacter`
  (params (Pawn :type "/Game/Blueprints/Pawns/TPCBP_Pawn Object Reference"))
  (`self.K2_TeleportTo` Pawn (+ (`self.K2_GetActorLocation`) (* (`self.GetActorRightVector`) -200.0)) (`KismetMathLibrary.MakeRotFromX` (`self.GetActorForwardVector`)))
  (`self.SetActorHiddenInGame` Pawn false)
  (bind _asplayer_controller (cast `PlayerController` (`self.GetController`)))
  (`Controller.Possess` _asplayer_controller Pawn))

(fn `GetPreviousCharacter`
  (returns (Pawn :type "/Game/Blueprints/Pawns/TPCBP_Pawn Object Reference") (Success :type Boolean))
  (locals (PreviousPawn :type "/Game/Blueprints/Pawns/TPCBP_Pawn Object Reference"))
  (bind _outactors (`GameplayStatics.GetAllActorsOfClass` "/Game/Blueprints/Pawns/TPCBP_Pawn.TPCBP_Pawn_C"))
  (for _array_element _outactors
    (if (== (`/Game/Blueprints/Pawns/TPCBP_Pawn.PreviousPlayerController` _array_element) (`self.GetController`))
      (set `local.PreviousPawn` _array_element)
      (break)))
  (bind _previouspawn (`local.PreviousPawn`)
    (:`then`
      (return _previouspawn true))
    (:`else`
      (return null false))))

(fn `UserConstructionScript`
  (`parent.UserConstructionScript`))