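; Player controller for the login screen, handling LAN session discovery, hosting and joining.
; On BeginPlay it shows the WBP_LogIn widget and cursor, then searches for sessions, displaying results or a hosting option if none are found or the search fails.
; Hosting creates a session and opens GameMap as a listen server.
; Joining uses either a selected session result or a console "open" command for a remote IP.
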(event `self.ReceiveBeginPlay`
  (bind _returnvalue (`|CreateWidget` "/Game/Blueprints/Widgets/WBP_LogIn.WBP_LogIn_C" self))
  (bind _output_get (set `self.LogInWidget` _returnvalue))
  (`UserWidget.AddToViewport` _output_get 0)
  (`self.OnSearchForHosts`)
  (set `self.bShowMouseCursor` true))

(event `/Game/Blueprints/Interfaces/IBP_PlayerController.OnJoinSession`
  (params (SessionResult :type "BlueprintSessionResult Structure"))
  (`JoinSessionCallbackProxy.JoinSession` self SessionResult))

(event `/Game/Blueprints/Interfaces/IBP_PlayerController.OnJoinRemoteSession`
  (params (IP :type String))
  (`KismetSystemLibrary.ExecuteConsoleCommand` (`KismetStringLibrary.Concat_StrStr` "open " IP) self))

(event `/Game/Blueprints/Interfaces/IBP_PlayerController.OnSearchForHosts`
  (bind _loginwidget (`self.LogInWidget`)
    (:`then`
      (`/Game/Blueprints/Widgets/WBP_LogIn.BeginSearchingForSessions` _loginwidget)
      (bind _results (`FindSessionsCallbackProxy.FindSessions` self 8 true)
        (:`OnSuccess`
          (if (> (`KismetArrayLibrary.Array_Length` _results) 0)
            (`/Game/Blueprints/Widgets/WBP_LogIn.DisplaySessions` (`self.LogInWidget`) _results)
            (else
              (`/Game/Blueprints/Widgets/WBP_LogIn.DisplayHosting` (`self.LogInWidget`) :!label _label))))
        (:`OnFailure`
          (goto _label))))
    (:`else`)))

(event `/Game/Blueprints/Interfaces/IBP_PlayerController.OnHostSession`
  (bind _loginwidget (`self.LogInWidget`)
    (:`then`
      (`/Game/Blueprints/Widgets/WBP_LogIn.HideHosting` _loginwidget)
      (`/Game/Blueprints/Widgets/WBP_LogIn.HideSessions` _loginwidget)
      (`/Game/Blueprints/Widgets/WBP_LogIn.BeginLoading` _loginwidget)
      (`CreateSessionCallbackProxy.CreateSession` self 7 false false
        (:`OnSuccess`
          (`GameplayStatics.OpenLevelBySoftObjectPtr` "/Game/Maps/GameMap.GameMap" true "?listen")
          (`Widget.SetVisibility` _loginwidget "Hidden"))))
    (:`else`)))

(fn `UserConstructionScript`)